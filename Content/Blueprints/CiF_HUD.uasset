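; CiF_HUD is a Blueprint that provides the UI layer for the CiF social simulation.
; On BeginPlay it builds and initializes a VM_SocialState view model from the CiF subsystem instance, using the buddy social network and all character objects.
; Separate functions create viewport widgets for the social state display and for character interactions, the latter receiving social games, an initiator and a responder.
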(event EventBeginPlay
  (bind _returnvalue (Class|CiFSubsystem|GetInstance (Subsystems|GetCiFSubsystem)))
  (bind _returnvalue_2 (Game|ConstructObjectfromClass "/CiF/Blueprints/UI/ViewModels/VM_SocialState.VM_SocialState_C" (Class|CiFManager|GetSocialNetworkbyType _returnvalue "BUDDY") (Class|CiFManager|GetAllGameObjectsOfType _returnvalue "CHARACTER")))
  (bind _output_get (Variables|Default|Setvm_cifSocialState _returnvalue_2))
  (Default|Init _output_get _returnvalue))

(event Collision|EventActorBeginOverlap
  (params (OtherActor :type Actor%20Object%20Reference)))

(event EventTick
  (params (DeltaSeconds :type Float%20%28single-precision%29)))

(fn ConstructionScript)

(fn CreateCharacterInteractionUI
  (params (socialGames :type Array%20of%20Social%20Game%20Intent%20Pair%20Structures) (initiator :type Cif%20NPC%20Object%20Reference) (responder :type Ci%20F%20Game%20Object%20Object%20Reference))
  (bind _returnvalue (UserInterface|CreateWidget "/CiF/Blueprints/UI/WBP_CharacterInteractionUI.WBP_CharacterInteractionUI_C" 0 socialGames initiator responder))
  (UserInterface|Viewport|AddtoViewport _returnvalue 0))

(fn CreateSocialStateUI
  (bind _returnvalue (UserInterface|CreateWidget "/CiF/Blueprints/UI/WBP_SocialState.WBP_SocialState_C"))
  (UserInterface|Viewport|AddtoViewport _returnvalue 0))