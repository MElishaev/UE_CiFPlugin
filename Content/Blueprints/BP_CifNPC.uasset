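; BP_CifNPC is an interactable NPC for the CiF social simulation demo, labeled with its character component's name via a text render.
; On Interact from the third-person player character, it asks the demo CiF implementation to prepare five social game options, with intent shown, between player and NPC.
; It then passes those options and both participants to the CiF HUD, which creates the character interaction UI.
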(event EventBeginPlay
  (Rendering|Components|TextRender|SetText (Variables|Default|GetTextRender) (Utilities|Text|ToText(Name) (Variables|/Script/CiF.CiFGameObject|GetmObjectName (Variables|Default|GetmCifCharacterComp))))
  (Utilities|IsValid (Variables|Default|GetmCifCharacterComp)
    (:Is%20Not%20Valid
      (Development|PrintString "character component isn't valid"))))

(event Collision|EventActorBeginOverlap
  (params (OtherActor :type Actor%20Object%20Reference)))

(event EventTick
  (params (DeltaSeconds :type Float%20%28single-precision%29)))

(event EventInteract
  (params (InstigatorPawn :type Pawn%20Object%20Reference) (HitResult :type Hit%20Result%20Structure))
  (bind _asbp_cif_third_person_character (Utilities|Casting|CastToBP_CifThirdPersonCharacter InstigatorPawn))
  (bind _asdemo_cif_implementation (Utilities|Casting|CastToDemoCifImplementation (Class|CiFSubsystem|GetImplementation (Subsystems|GetCiFSubsystem))))
  (bind _outsocialgamesnames (Class|DemoCifImplementation|PrepareSocialGameOptionswithCharacter _asdemo_cif_implementation _asbp_cif_third_person_character (Variables|Default|GetmCifCharacterComp) 5 true false))
  ;[1 1 1] show character interaction UI
  (bind _asci_f_hud (Utilities|Casting|CastToBP_Cif_HUD (HUD|GetHUD (Game|GetPlayerController 0))))
  (Default|CreateCharacterInteractionUI _asci_f_hud _outsocialgamesnames _asbp_cif_third_person_character (Variables|Default|GetmCifCharacterComp)))

(fn ConstructionScript)