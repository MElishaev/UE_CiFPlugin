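; Game mode Blueprint that sets up the Cif system and populates the level with its cast of NPCs.
; On BeginPlay it initializes Cif, then spawns a BP_CifNPC for every character in the Cif manager's cast except the one named "Player".
; Each NPC receives its character component, appears at a random reachable navigation point around a hard-coded origin, and is added to the NPC list.
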(event EventBeginPlay
  (Class|CiFGameMode|InitCif)
  (Class|CiFGameMode|SpawnCastinLevel))

(event EventSpawnCastinLevel
  (CallFunction|SpawnCastinLevelBP))

(fn ConstructionScript)

(fn SpawnCastinLevelBP
  (for _array_element (Variables|/Script/CiF.CiFCast|GetmCharacters (Variables|/Script/CiF.CiFManager|GetmCast (Variables|Default|GetmCifManager)))
    (if (!= (Variables|/Script/CiF.CiFGameObject|GetmObjectName _array_element) "Player")
      (bind _returnvalue (Game|SpawnActorfromClass "/CiF/Blueprints/BP_CifNPC.BP_CifNPC_C" (Math|Transform|MakeTransform (.RandomLocation (AI|Navigation|GetRandomReachablePointinRadius (Math|Vector|MakeVector 1.3e+02 5.8e+02 725.0) 7e+02 0 0)) "0, 0, 0" "1.000000,1.000000,1.000000") "AdjustIfPossibleButDontSpawnIfColliding" "MultiplyWithRoot" 0 _array_element 0))
      (Utilities|Array|Add (Variables|Default|GetmCifNPCs) _returnvalue))))