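; Game mode that boots the CiF subsystem and populates the level with its cast of NPCs.
; On BeginPlay it initializes the CiF manager and installs a DemoCifImplementation on the subsystem.
; It then spawns a BP_CifNPC for each non-Player cast character at a random reachable point around a hardcoded origin, passing in that character's data.
; Spawned NPCs are tracked in an array for lookup by name.
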(event EventBeginPlay
  (CallFunction|InitCif)
  (CallFunction|SpawnCastinLevel))

(fn ConstructionScript)

(fn SpawnCastinLevel
  (for _array_element (Variables|/Script/CiF.CiFCast|GetmCharacters (Variables|/Script/CiF.CiFManager|GetmCast (Variables|Default|GetCif%20Manager)))
    (if (!= (Variables|/Script/CiF.CiFGameObject|GetmObjectName _array_element) "Player")
      (bind _returnvalue (Game|SpawnActorfromClass "/CiF/Blueprints/BP_CifNPC.BP_CifNPC_C" (Math|Transform|MakeTransform (.RandomLocation (AI|Navigation|GetRandomReachablePointinRadius (Math|Vector|MakeVector 8e+01 5.8e+02 725.0626) 7e+02 0 0)) "0, 0, 0" "1.000000,1.000000,1.000000") "AdjustIfPossibleButDontSpawnIfColliding" "MultiplyWithRoot" 0 _array_element 0))
      (Utilities|Array|Add (Variables|Default|GetcifNPCs) _returnvalue))))

(fn InitCif
  (bind _returnvalue (Subsystems|GetCiFSubsystem))
  (bind _returnvalue_2 (Class|CiFSubsystem|GetInstance _returnvalue))
  (bind _output_get (Variables|Default|SetCif%20Manager _returnvalue_2))
  (Class|CiFManager|Init _output_get)
  (bind _returnvalue_3 (Game|ConstructObjectfromClass "/Script/CiF.DemoCifImplementation"))
  (Utilities|IsValid _returnvalue_3
    (:Is%20Valid
      (Class|CiFSubsystem|SetImplementation _returnvalue _returnvalue_3))
    (:Is%20Not%20Valid
      (Development|PrintString "cif implementation isnt valid"))))

(fn GetCifNPCbyName
  (params (name :type Name))
  (for _array_element (Variables|Default|GetcifNPCs)
    (if (== (Variables|/Script/CiF.CiFGameObject|GetmObjectName (Variables|/Script/CiF.CifNPC|GetmCifCharacterComp _array_element)) name)
      (return _array_element)))
  (Development|PrintString (Utilities|String|Append (Utilities|String|MakeLiteralString "couldn't find ") (Utilities|String|ToString(Name) name)))
  (return 0))