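; HUD for the CiF social simulation that owns the view models and spawns the game's UI widgets.
; BeginPlay builds social state and task assignment view models from the CiF instance, plus a resources view model from the game state's resource manager.
; It shows the resource bar immediately.
; Separate functions open social state, task assignment and character interaction widgets, passing the task view model or interaction participants where needed.
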(event EventBeginPlay
  (bind _returnvalue (Class|CiFSubsystem|GetInstance (Subsystems|GetCiFSubsystem)))
  (Utilities|FlowControl|Sequence
    (:then_0
      (bind _returnvalue_2 (Game|ConstructObjectfromClass "/CiF/Blueprints/UI/ViewModels/VM_SocialState.VM_SocialState_C" (Class|CiFManager|GetSocialNetworkbyType _returnvalue "BUDDY") (Class|CiFManager|GetAllGameObjectsOfType _returnvalue "CHARACTER")))
      (bind _output_get (Variables|Default|Setvm_cifSocialState _returnvalue_2))
      (Default|Init _output_get _returnvalue))
    (:then_1
      (bind _returnvalue_3 (Game|ConstructObjectfromClass "/Game/Blueprints/UI/TaskAssignment/VM_TaskAssignment.VM_TaskAssignment_C" _returnvalue))
      (bind _output_get_2 (Variables|Default|Setvm_taskAssignment _returnvalue_3))
      (Default|Init _output_get_2))
    (:then_2
      (bind _returnvalue_4 (Game|ConstructObjectfromClass "/Game/Blueprints/UI/Resources/VM_Resources.VM_Resources_C"))
      (bind _output_get_3 (Variables|Default|Setvm_resourceBar _returnvalue_4))
      (bind _asbp_game_state (Utilities|Casting|CastToBP_GameState (Game|GetGameState)))
      (Default|Init _output_get_3 (Variables|/Script/CiFPrototype.MK_ResourceManager|GetmResourcesMap (Variables|/Script/CiFPrototype.MK_GameState|GetmResourceManager _asbp_game_state)))
      (CallFunction|CreateandShowResourcesBar))))

(event Collision|EventActorBeginOverlap
  (params (OtherActor :type Actor%20Object%20Reference)))

(event EventTick
  (params (DeltaSeconds :type Float%20%28single-precision%29)))

(fn ConstructionScript)

(fn CreateCharacterInteractionUI
  (params (socialGames :type Array%20of%20Social%20Game%20Intent%20Pair%20Structures) (initiator :type Cif%20NPC%20Object%20Reference) (responder :type Ci%20F%20Game%20Object%20Object%20Reference))
  (bind _returnvalue (UserInterface|CreateWidget "/CiF/Blueprints/UI/WBP_CharacterInteractionUI.WBP_CharacterInteractionUI_C" 0 socialGames initiator responder))
  (UserInterface|Viewport|AddtoViewport _returnvalue 0))

(fn CreateandShowSocialStateUI
  (bind _returnvalue (UserInterface|CreateWidget "/CiF/Blueprints/UI/WBP_SocialState.WBP_SocialState_C"))
  (UserInterface|Viewport|AddtoViewport _returnvalue 0))

(fn CreateandShowTaskAssignmentUI
  (bind _returnvalue (UserInterface|CreateWidget "/Game/Blueprints/UI/TaskAssignment/WBP_MainTaskAssignment.WBP_MainTaskAssignment_C" 0 (Variables|Default|Getvm_taskAssignment)))
  (UserInterface|Viewport|AddtoViewport _returnvalue 0))

(fn CreateandShowResourcesBar
  (bind _returnvalue (UserInterface|CreateWidget "/Game/Blueprints/UI/Resources/WBP_ResourceBar.WBP_ResourceBar_C" 0 (Variables|Default|Getvm_resourceBar)))
  (UserInterface|Viewport|AddtoViewport _returnvalue 0))